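; Toilet actor that the third-person player uses when ready to poo.
; On Interact press, if the toilet is Activated and the character's ReadyToPoo flag is set, it plays a flush sound at the mesh.
; It then calls PooMessage on the character, passing a transform offset above and in front of the toilet's root, facing the root's rotation.
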(event EventBeginPlay
  (|CallParentFunction) ; This node is disabled and will not be called.\nDrag off pins to build functionality.
)

(event Input|ActionEvents|InputActionInteract
  (params (Key :type Key%20Structure :default "None"))
  (bind _defaultsceneroot (Variables|Default|GetDefaultSceneRoot))
  (bind _returnvalue (Transformation|GetWorldRotation _defaultsceneroot))
  (:Pressed
    (bind _asthird_person_character (Utilities|Casting|CastToThirdPersonCharacter (Game|GetPlayerCharacter 0)))
    (if (Variables|Default|Getactivated)
      (if (Variables|/Game/ThirdPersonBP/Blueprints/ThirdPersonCharacter.ThirdPersonCharacter_C|GetreadyToPoo _asthird_person_character)
        (Audio|PlaySoundatLocation "/Game/Sound/toilet_flush_sound.toilet_flush_sound" (Transformation|GetWorldLocation (Variables|Default|GetStaticMesh)) "0, 0, 0" 1.0 1.0 0.0 0 0 0)
        (Class|CatInterface|Poo(Message) _asthird_person_character (Math|Transform|MakeTransform (+ (+ (Transformation|GetWorldLocation _defaultsceneroot) "0.000000, 0,120.000000") (* (Math|Vector|GetForwardVector _returnvalue) 1e+02)) _returnvalue))))))

(fn ConstructionScript
  (|CallParentFunction))