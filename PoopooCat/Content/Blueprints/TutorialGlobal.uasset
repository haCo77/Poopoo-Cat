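; TutorialGlobal runs the tutorial flow, showing instruction messages, tracking the level and handling pause.
; BeginPlay resets the level and shows the TutorialUI movement message; the Pause input opens PauseMenu once, guarded by a flag.
; Each LevelUp spawns scaled-down Food above the player, offset along the mesh's forward vector, and reaching level two triggers the digest message.
; Creation of the DigestBarNFoodReq and CompassBar widgets is left unconnected.
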(event EventBeginPlay
  (Variables|Default|Setlevel 0)
  (bind _returnvalue (Game|ConstructObjectfromClass "/Game/UI/TutorialUI.TutorialUI_C" (Game|GetPlayerController 0)))
  (UserInterface|Viewport|AddtoViewport _returnvalue 0)
  (Class|Tutorial|ShowMoveInc(Message) _returnvalue))

(event Collision|EventActorBeginOverlap
  (params (OtherActor :type Actor%20Object%20Reference)))

(event EventTick
  (params (DeltaSeconds :type Float%20%28single-precision%29)))

(event EventLevelUp
  (bind _returnvalue (Game|GetPlayerCharacter 0))
  (Game|SpawnActorfromClass "/Game/Blueprints/Food.Food_C" (Math|Transform|MakeTransform (+ (Transformation|GetActorLocation _returnvalue) (+ (* (Math|Vector|GetForwardVector (Variables|/Script/Engine.Character|GetMesh _returnvalue)) 2e+02) "0, 0,200.000000")) "0, 0, 0" "0.300000,0.300000,0.300000") "Undefined" 0 0)
  (Variables|Default|Setlevel (+ (Variables|Default|Getlevel) 1))
  (if (== (Variables|Default|Getlevel) 2)
    (bind _foundwidgets (Widget|GetAllWidgetsOfClass "/Game/UI/TutorialUI.TutorialUI_C" true))
    (Class|Tutorial|ShowDigestInc(Message) (Utilities|Array|Get(acopy) _foundwidgets))))

(event Input|ActionEvents|InputActionPause
  (params (Key :type Key%20Structure :default "None"))
  (:Pressed
    (if (not (Variables|Default|Getpause_flag))
      (bind _returnvalue (UserInterface|CreateWidget "/Game/UI/PauseMenu.PauseMenu_C"))
      (UserInterface|Viewport|AddtoViewport _returnvalue 0)
      (Variables|/Script/Engine.PlayerController|SetbShowMouseCursor (Game|GetPlayerController 0) true)
      (Variables|Default|Setpause_flag true)
      (Game|SetGamePaused true))))

(fn ConstructionScript)