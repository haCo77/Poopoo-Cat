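; Food Blueprint for an item that the TopDownCharacter picks up and carries on its head.
; Clicking its sphere or pressing Interact while Activated tells the character to put down food it already holds, or to pick up this one.
; Pickup attaches the food to the mesh's head socket, marks it held and disabled, and hides its widget.
; Enablefood resets only the held and enabled flags.
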(event OnClicked(Sphere1)
  (params (TouchedComponent :type Primitive%20Component%20Object%20Reference) (ButtonPressed :type Key%20Structure :default "None"))
  (bind _self self)
  (if (Variables|Default|Getactivated)
    (bind _astop_down_character (Utilities|Casting|CastToTopDownCharacter (Game|GetPlayerCharacter 0)))
    (if (Variables|/Game/TopDownBP/Blueprints/TopDownCharacter.TopDownCharacter_C|Getholdingfood _astop_down_character)
      (Class|Interactions|PutDownFood(Message) _astop_down_character)
      (else
        (Class|Interactions|PickUpFood(Message) _astop_down_character _self)
        (Transformation|AttachComponentToComponent _self (Variables|/Script/Engine.Character|GetMesh _astop_down_character) "head" "SnapToTarget" "KeepRelative" "KeepWorld" true)
        (Variables|Default|Setbeingheld true)
        (Variables|Default|SetEnabled false)
        (Rendering|SetVisibility (Variables|Default|GetWidget) false false)))))

(event EventBeginPlay
  (|CallParentFunction) ; This node is disabled and will not be called.\nDrag off pins to build functionality.
)

(event EventEnablefood
  (Variables|Default|Setbeingheld false)
  (Variables|Default|SetEnabled true))

(event Input|ActionEvents|InputActionInteract
  (params (Key :type Key%20Structure :default "None"))
  (bind _self self)
  (:Pressed
    (if (Variables|Default|Getactivated)
      (bind _astop_down_character (Utilities|Casting|CastToTopDownCharacter (Game|GetPlayerCharacter 0)))
      (if (Variables|/Game/TopDownBP/Blueprints/TopDownCharacter.TopDownCharacter_C|Getholdingfood _astop_down_character)
        (Class|Interactions|PutDownFood(Message) _astop_down_character)
        (else
          (Class|Interactions|PickUpFood(Message) _astop_down_character _self)
          (Transformation|AttachComponentToComponent _self (Variables|/Script/Engine.Character|GetMesh _astop_down_character) "head" "SnapToTarget" "KeepRelative" "KeepWorld" true)
          (Variables|Default|Setbeingheld true)
          (Variables|Default|SetEnabled false)
          (Rendering|SetVisibility (Variables|Default|GetWidget) false false))))))

(fn ConstructionScript
  (|CallParentFunction))